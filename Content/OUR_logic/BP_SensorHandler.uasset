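; BP_SensorHandler is a sensor that briefly shows its Places component when a movable component overlaps its Box.
; Tick polls SensorHandler's mobility and, once it reads Stationary with Start set, activates the sensor, unhides Places and makes Places and Box Stationary.
; While active, a movable overlap makes Places visible for a short delay, and ending the overlap hides it immediately.
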(event `self.ReceiveTick`
  (params (DeltaSeconds :type "Float (single-precision)"))
  (bind _places (`self.Places`))
  (if (== (enumliteral `EComponentMobility` "Stationary") (`SceneComponent.Mobility` (`self.SensorHandler`)))
    (if (`self.start`)
      (set `self.Is_Active` true)
      (`SceneComponent.SetHiddenInGame` _places false false)
      (`SceneComponent.SetMobility` _places "Stationary")
      (`SceneComponent.SetMobility` (`self.Box`) "Stationary")
      (set `self.start` false))))

(event `self.Box.OnComponentBeginOverlap`
  (params (OverlappedComponent :type "PrimitiveComponent Object Reference") (OtherActor :type "Actor Object Reference") (OtherComp :type "PrimitiveComponent Object Reference") (OtherBodyIndex :type Integer) (bFromSweep :type Boolean) (SweepResult :type "HitResult Structure (by ref)"))
  (bind _places (`self.Places`))
  (if (`self.Is_Active`)
    (if (== (`SceneComponent.Mobility` OtherComp) (enumliteral `EComponentMobility` "Movable"))
      (`SceneComponent.SetVisibility` _places true false)
      (`KismetSystemLibrary.Delay` 2.0)
      (`SceneComponent.SetVisibility` _places false false :!label _label))))

(event `self.Box.OnComponentEndOverlap`
  (params (OverlappedComponent :type "PrimitiveComponent Object Reference") (OtherActor :type "Actor Object Reference") (OtherComp :type "PrimitiveComponent Object Reference") (OtherBodyIndex :type Integer))
  (if (`self.Is_Active`)
    (if (== (`SceneComponent.Mobility` OtherComp) (enumliteral `EComponentMobility` "Movable"))
      (goto _label))))

(fn `UserConstructionScript`)