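; BP_base_of_dron is a Blueprint, named as a drone base, built from Cube, Sphere and Cube1 components.
; On BeginPlay it sets all three components to Movable.
; Sphere overlap events check whether the other component is Movable, then set Cube1's visibility without propagating to children.
; Both begin and end overlap hide Cube1, so nothing in this graph makes it visible again.
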(event `self.ReceiveBeginPlay`
  (`SceneComponent.SetMobility` (`self.Cube`) "Movable")
  (`SceneComponent.SetMobility` (`self.Sphere`) "Movable")
  (`SceneComponent.SetMobility` (`self.Cube1`) "Movable"))

(event `self.Sphere.OnComponentBeginOverlap`
  (params (OverlappedComponent :type "PrimitiveComponent Object Reference") (OtherActor :type "Actor Object Reference") (OtherComp :type "PrimitiveComponent Object Reference") (OtherBodyIndex :type Integer) (bFromSweep :type Boolean) (SweepResult :type "HitResult Structure (by ref)"))
  (if (== (`SceneComponent.Mobility` OtherComp) (enumliteral `EComponentMobility` "Movable"))
    (`SceneComponent.SetVisibility` (`self.Cube1`) false false)))

(event `self.Sphere.OnComponentEndOverlap`
  (params (OverlappedComponent :type "PrimitiveComponent Object Reference") (OtherActor :type "Actor Object Reference") (OtherComp :type "PrimitiveComponent Object Reference") (OtherBodyIndex :type Integer))
  (if (== (`SceneComponent.Mobility` OtherComp) (enumliteral `EComponentMobility` "Movable"))
    (`SceneComponent.SetVisibility` (`self.Cube1`) false false)))

(fn `UserConstructionScript`)