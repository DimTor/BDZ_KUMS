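; Player character with a visible mouse cursor that walks, flies vertically and drags objects in the world.
; Standard axes handle movement and look; held Q/E shift the capsule down/up each Tick, and right mouse enables camera pitching.
; When GrabMode is on, left mouse traces under the cursor for Movable components.
; Tick holds the grabbed component at its original distance along the cursor ray, using PhysicsHandle for simulated bodies and SetWorldLocation otherwise.
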(event `self.ReceiveTick`
  (params (DeltaSeconds :type "Float (single-precision)"))
  (bind _grab_component (`self.Grab_component`))
  (bind _capsulecomponent (`self.CapsuleComponent`))
  (bind _camera (`self.Camera`))
  (bind (_worldlocation _worlddirection) (`PlayerController.DeprojectMousePositionToWorld` (`GameplayStatics.GetPlayerController` 0)))
  (bind (_relativerotation_roll _relativerotation_pitch) (`KismetMathLibrary.BreakRotator` (`SceneComponent.RelativeRotation` _camera)))
  (bind (_relativelocation_x _relativelocation_y _relativelocation_z) (`KismetMathLibrary.BreakVector` (`SceneComponent.RelativeLocation` _capsulecomponent)))
  (bind (_relativelocation_x_2 _relativelocation_y_2 _relativelocation_z_2) (`KismetMathLibrary.BreakVector` (`SceneComponent.RelativeLocation` _capsulecomponent)))
  (bind _returnvalue (+ _worldlocation (* _worlddirection (`self.OriginalDistanceToObject`))))
  (if (`self.Q_ok`)
    (`SceneComponent.K2_SetRelativeLocation` _capsulecomponent (`KismetMathLibrary.MakeVector` _relativelocation_x _relativelocation_y (- _relativelocation_z (`self.speed`))) false false))
  (if (`self.E_ok`)
    (`SceneComponent.K2_SetRelativeLocation` _capsulecomponent (`KismetMathLibrary.MakeVector` _relativelocation_x_2 _relativelocation_y_2 (+ _relativelocation_z_2 (`self.speed`))) false false))
  (if (`self.Right_Ok`)
    (`SceneComponent.K2_SetRelativeRotation` _camera (`KismetMathLibrary.MakeRotator` 0.0 (+ (* (`self.GetInputAxisKeyValue`) 3.0) _relativerotation_pitch)) false false))
  (if (`self.Grab_Mode`)
    (if (`KismetSystemLibrary.IsValid` _grab_component)
      (if (`SceneComponent.IsSimulatingPhysics` _grab_component "None")
        (`PhysicsHandleComponent.SetTargetLocation` (`self.PhysicsHandle`) _returnvalue)
        (else
          (`SceneComponent.K2_SetWorldLocation` (`self.Grab_component`) _returnvalue false false))))))

(event `Key|LeftMouseButton`
  (params (Key :type "Key Structure"))
  (bind _grab_mode (`self.Grab_Mode`))
  (bind (_worldlocation _worlddirection) (`PlayerController.DeprojectMousePositionToWorld` (`GameplayStatics.GetPlayerController` 0)))
  (:`Pressed`
    (if _grab_mode
      (bind _outhit (`KismetSystemLibrary.LineTraceSingle` :`Start` _worldlocation :`End` (+ _worldlocation (* _worlddirection 1000.0)) :`TraceChannel` "TraceTypeQuery1" :`DrawDebugType` "ForDuration" :`DrawTime` 2.0))
      (bind (_bblockinghit _binitialoverlap _time _distance _location _impactpoint _normal _impactnormal _physmat _hitactor _hitcomponent) (`GameplayStatics.BreakHitResult` _outhit))
      (if (`KismetSystemLibrary.IsValid` _hitcomponent)
        (if (`|EnumEquality` (`SceneComponent.Mobility` _hitcomponent) (enumliteral `EComponentMobility` "Movable"))
          (`KismetSystemLibrary.PrintString` "Ok")
          (bind _output_get (set `self.Grab_component` _hitcomponent))
          (set `self.OriginalDistanceToObject` _distance)
          (if (`SceneComponent.IsSimulatingPhysics` _output_get "None")
            (`PhysicsHandleComponent.GrabComponentAtLocation` (`self.PhysicsHandle`) (`self.Grab_component`) "None" _location)
            (else
              (set `self.RelativeGrabLocation` (`KismetMathLibrary.InverseTransformLocation` (`KismetMathLibrary.Conv_VectorToTransform` _location) (`SceneComponent.K2_GetComponentLocation` _hitcomponent)))))
          (else
            (`KismetSystemLibrary.PrintString` "Stationary")))
        (else
          (`KismetSystemLibrary.PrintString` "Hello")))))
  (:`Released`
    (if _grab_mode
      (set `self.Grab_component` null)
      (`PhysicsHandleComponent.ReleaseComponent` (`self.PhysicsHandle`)))))

(event `self.ReceiveBeginPlay`
  (set `PlayerController.bShowMouseCursor` true (`GameplayStatics.GetPlayerController` 0)))

(event `Key|E`
  (params (Key :type "Key Structure"))
  (:`Pressed`
    (set `self.E_ok` true))
  (:`Released`
    (set `self.E_ok` false)))

(event `Key|Q`
  (params (Key :type "Key Structure"))
  (:`Pressed`
    (set `self.Q_ok` true))
  (:`Released`
    (set `self.Q_ok` false)))

(event `InputAxis|TurnRate`
  (params (AxisValue :type "Float (single-precision)"))
  (`self.AddControllerYawInput` (* AxisValue (`self.BaseTurnRate`) (`GameplayStatics.GetWorldDeltaSeconds`))))

(event `InputAxis|LookUpRate`
  (params (AxisValue :type "Float (single-precision)"))
  (`self.AddControllerPitchInput` (* AxisValue (`self.BaseLookUpRate`) (`GameplayStatics.GetWorldDeltaSeconds`))))

(event `InputAction|ResetVR`
  (params (Key :type "Key Structure"))
  (:`Pressed`
    (`HeadMountedDisplayFunctionLibrary.ResetOrientationAndPosition` 0.0)))

(event `InputAxis|Turn` :overrideparent false
  (params (AxisValue :type "Float (single-precision)"))
  (`self.AddControllerYawInput` AxisValue))

(event `InputAxis|MoveForward` :overrideparent false
  (params (AxisValue :type "Float (single-precision)"))
  (`self.AddMovementInput` (`KismetMathLibrary.GetForwardVector` (`KismetMathLibrary.MakeRotator` 0.0 0.0 (.yaw (`self.GetControlRotation`)))) AxisValue))

(event `Key|RightMouseButton`
  (params (Key :type "Key Structure"))
  (:`Pressed`
    (set `self.Right_Ok` true))
  (:`Released`
    (set `self.Right_Ok` false)))

(event `InputAxis|MoveRight` :overrideparent false
  (params (AxisValue :type "Float (single-precision)"))
  (`self.AddMovementInput` (`KismetMathLibrary.GetRightVector` (`KismetMathLibrary.MakeRotator` 0.0 0.0 (.yaw (`self.GetControlRotation`)))) AxisValue))

(fn `UserConstructionScript`)