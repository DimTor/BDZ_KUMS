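; BP_motor is a motor part in a drone assembly task that accepts a BP_wheels attachment and ends the game when it is fitted.
; Tick activates the socket once the motor is Stationary, and Box overlaps toggle the Places marker for Movable components.
; Movable wheels hitting visible Places snap there, rotate by side relative to BP_base_of_dron, lock Stationary and call EndOfGame on BP_character.
; BP_ved_wheels instead triggers MakeMistake.
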(event `self.ReceiveTick`
  (params (DeltaSeconds :type "Float (single-precision)"))
  (bind _places (`self.Places`))
  (if (== (enumliteral `EComponentMobility` "Stationary") (`SceneComponent.Mobility` (`self.Motor`)))
    (if (`self.start`)
      (set `self.is_active` true)
      (`SceneComponent.SetHiddenInGame` _places false false)
      (`SceneComponent.SetMobility` _places "Stationary")
      (`SceneComponent.SetMobility` (`self.Box`) "Stationary")
      (set `self.start` false))))

(event `self.Box.OnComponentBeginOverlap`
  (params (OverlappedComponent :type "PrimitiveComponent Object Reference") (OtherActor :type "Actor Object Reference") (OtherComp :type "PrimitiveComponent Object Reference") (OtherBodyIndex :type Integer) (bFromSweep :type Boolean) (SweepResult :type "HitResult Structure (by ref)"))
  (bind _places (`self.Places`))
  (if (`self.is_active`)
    (if (== (`SceneComponent.Mobility` OtherComp) (enumliteral `EComponentMobility` "Movable"))
      (`SceneComponent.SetVisibility` _places true false)
      (`KismetSystemLibrary.Delay` 2.0)
      (`SceneComponent.SetVisibility` _places false false :!label _label))))

(event `self.Places.OnComponentBeginOverlap`
  (params (OverlappedComponent :type "PrimitiveComponent Object Reference") (OtherActor :type "Actor Object Reference") (OtherComp :type "PrimitiveComponent Object Reference") (OtherBodyIndex :type Integer) (bFromSweep :type Boolean) (SweepResult :type "HitResult Structure (by ref)"))
  (bind (_returnvalue_x _returnvalue_y) (`KismetMathLibrary.BreakVector` (`SceneComponent.K2_GetComponentLocation` (`self.Motor`))))
  (if (`self.is_active`)
    (if (`SceneComponent.IsVisible` OtherComp)
      (if (== (`SceneComponent.Mobility` OtherComp) (enumliteral `EComponentMobility` "Movable"))
        (bind _returnvalue (`GameplayStatics.GetActorOfClass` "/Game/OUR_logic/BP_wheels.BP_wheels_C"))
        (if (== (`GameplayStatics.GetObjectClass` _returnvalue) (`GameplayStatics.GetObjectClass` OtherActor))
          (`SceneComponent.K2_SetWorldLocation` OtherComp (`SceneComponent.K2_GetComponentLocation` (`self.Places`)) false false)
          (bind _returnvalue_2 (`GameplayStatics.GetActorOfClass` "/Game/OUR_logic/BP_base_of_dron.BP_base_of_dron_C"))
          (bind (_returnvalue_x_2 _returnvalue_y_2) (`KismetMathLibrary.BreakVector` (`SceneComponent.K2_GetComponentLocation` (`/Game/OUR_logic/BP_base_of_dron.Places3` _returnvalue_2))))
          (if (> _returnvalue_y_2 _returnvalue_y)
            (`SceneComponent.K2_SetWorldRotation` OtherComp (struct :`Pitch` 90.0) false false)
            (else
              (`SceneComponent.K2_SetWorldRotation` OtherComp (struct :`Pitch` -90.0 :`Yaw` 180.0) false false)))
          (if true
            (`SceneComponent.SetMobility` (`Actor.RootComponent` OtherActor) "Stationary")
            (set `self.is_active` false)
            (`SceneComponent.SetVisibility` (`self.Places`) false false)
            (bind _returnvalue_3 (`GameplayStatics.GetActorOfClass` "/Game/OUR_logic/BP_character.BP_character_C"))
            (`/Game/OUR_logic/BP_character.End_of_game` _returnvalue_3))
          (else
            (bind _returnvalue_4 (`GameplayStatics.GetActorOfClass` "/Game/OUR_logic/BP_ved_wheels.BP_ved_wheels_C"))
            (if (== (`GameplayStatics.GetObjectClass` _returnvalue_4) (`GameplayStatics.GetObjectClass` OtherActor))
              (bind _returnvalue_5 (`GameplayStatics.GetActorOfClass` "/Game/OUR_logic/BP_character.BP_character_C"))
              (`/Game/OUR_logic/BP_character.Make_mistake` _returnvalue_5))))))))

(event `self.Box.OnComponentEndOverlap`
  (params (OverlappedComponent :type "PrimitiveComponent Object Reference") (OtherActor :type "Actor Object Reference") (OtherComp :type "PrimitiveComponent Object Reference") (OtherBodyIndex :type Integer))
  (if (`self.is_active`)
    (if (== (`SceneComponent.Mobility` OtherComp) (enumliteral `EComponentMobility` "Movable"))
      (goto _label))))

(fn `UserConstructionScript`)