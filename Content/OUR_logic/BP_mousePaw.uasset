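; BP_mousePaw is an early mouse-interaction Blueprint that toggles the cursor and casts a debug trace from it into the world.
; The T key flips cursor visibility on the first player controller.
; Left mouse press and release share one path that prints debug text and, when GrabMode is set, line traces along the deprojected cursor direction on the Visibility channel.
; The trace result is unused, so nothing is grabbed yet.
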(event `Key|T`
  (params (Key :type "Key Structure"))
  (bind _returnvalue (`GameplayStatics.GetPlayerController` 0))
  (:`Pressed`
    (set `PlayerController.bShowMouseCursor` (not (`PlayerController.bShowMouseCursor` _returnvalue)) _returnvalue)))

(event `Key|LeftMouseButton`
  (params (Key :type "Key Structure"))
  (bind (_worldlocation _worlddirection) (`PlayerController.DeprojectMousePositionToWorld` (`GameplayStatics.GetPlayerController` 0)))
  (:`Pressed`
    (`KismetSystemLibrary.PrintString` "Hello" :!label _label)
    (if (`self.grab_mode`)
      (`KismetSystemLibrary.PrintString` "Hello")
      (`KismetSystemLibrary.LineTraceSingle` :`Start` _worldlocation :`End` (+ _worldlocation (* _worlddirection 1000.0)) :`TraceChannel` "TraceTypeQuery1" :`DrawDebugType` "ForDuration")))
  (:`Released`
    (goto _label)))

(fn `UserConstructionScript`)