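; 3D printer actor that prints batches of six part types, animating the printer and spawning each piece at its root.
; BeginPlay resets the game instance's detail counts and shows an introduction widget; OK opens the printing menu.
; 3D-printing runs chained DoN loops, one per Detail count, with a timed delay per piece, skipping zero counts and re-showing the menu afterwards.
; The V key hides that menu for a pause widget, and ClosePause restores it.
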(event `Close Pause`
  (`Widget.SetVisibility` (stale `OK` _returnvalue) "Visible"))

(event `Key|V`
  (params (Key :type "Key Structure"))
  (:`Pressed`
    (`Widget.SetVisibility` (stale `OK` _returnvalue) "Hidden")
    (if (`self.Pause`)
      (`Widget.SetVisibility` (stale _returnvalue) "Visible")
      (else
        (bind _returnvalue (`|CreateWidget` "/Game/OUR_logic/BP_Pause.BP_Pause_C"))
        (`UserWidget.AddToViewport` _returnvalue 0)
        (set `self.Pause` true)))))

(event `self.ReceiveBeginPlay`
  (bind _asbp_instance (cast `/Game/OUR_logic/BP_Instance` (`GameplayStatics.GetGameInstance`)))
  (set `/Game/OUR_logic/BP_Instance.Scene` 2 _asbp_instance)
  (set `/Game/OUR_logic/BP_Instance.Detail_1` 0 _asbp_instance)
  (set `/Game/OUR_logic/BP_Instance.Detail_2` 0 _asbp_instance)
  (set `/Game/OUR_logic/BP_Instance.Detail_3` 0 _asbp_instance)
  (set `/Game/OUR_logic/BP_Instance.Detail_4` 0 _asbp_instance)
  (set `/Game/OUR_logic/BP_Instance.Detail_5` 0 _asbp_instance)
  (set `/Game/OUR_logic/BP_Instance.Detail_6` 0 _asbp_instance)
  (set `/Game/OUR_logic/BP_Instance.Scene` 1 _asbp_instance)
  (bind _returnvalue (`|CreateWidget` "/Game/OUR_logic/BP_Introduction.BP_Introduction_C"))
  (`UserWidget.AddToViewport` _returnvalue 0))

(event `OK`
  (bind _returnvalue (`|CreateWidget` "/Game/OUR_logic/BP_Printing_Menu.BP_Printing_Menu_C"))
  (`UserWidget.AddToViewport` _returnvalue 0))

(event `3D-printing`
  (bind _detail_6 (`self.detail_6`))
  (bind _detail_2 (`self.detail_2`))
  (bind _detail_3 (`self.detail_3`))
  (bind _detail_4 (`self.detail_4`))
  (bind _detail_5 (`self.detail_5`))
  (bind _detail_1 (`self.detail_1`))
  (`self.Reset_loop`)
  (if (!= _detail_1 0)
    (bind _counter (`/Engine/EditorBlueprintResources/StandardMacros.Do N` _detail_1 :!label _label)
      (:`Exit`
        (`SkeletalMeshComponent.PlayAnimation` (`self.3D-printer`) "/Game/OUR_models/3D-printer/3D-printer_Anim.3D-printer_Anim" false)
        (`|SpawnActorFromClass` "/Game/OUR_logic/Printing_models/BP_MainPlate.BP_MainPlate_C" (`SceneComponent.K2_GetComponentToWorld` (`self.DefaultSceneRoot`)) "Undefined" "OverrideRootScale" null null)
        (`KismetSystemLibrary.Delay` 4.3)
        (`SkeletalMeshComponent.Stop` (`self.3D-printer`))
        (`KismetSystemLibrary.PrintString` "stop")
        (if (== _counter _detail_1)
          _
          (else
            (goto _label))))))
  (if (!= _detail_2 0)
    (bind _counter_2 (`/Engine/EditorBlueprintResources/StandardMacros.Do N` _detail_2 :!label _label_2)
      (:`Exit`
        (`SkeletalMeshComponent.PlayAnimation` (`self.3D-printer`) "/Game/OUR_models/3D-printer/3D-printer_Anim.3D-printer_Anim" false)
        (`|SpawnActorFromClass` "/Game/OUR_logic/Printing_models/BP_SensorHandler.BP_SensorHandler_C" (`SceneComponent.K2_GetComponentToWorld` (`self.DefaultSceneRoot`)) "Undefined" "OverrideRootScale" null null)
        (`KismetSystemLibrary.Delay` 4.3)
        (`SkeletalMeshComponent.Stop` (`self.3D-printer`))
        (`KismetSystemLibrary.PrintString` "stop")
        (if (== _counter_2 _detail_2)
          _
          (else
            (goto _label_2))))))
  (if (!= _detail_3 0)
    (bind _counter_3 (`/Engine/EditorBlueprintResources/StandardMacros.Do N` _detail_3 :!label _label_3)
      (:`Exit`
        (`SkeletalMeshComponent.PlayAnimation` (`self.3D-printer`) "/Game/OUR_models/3D-printer/3D-printer_Anim.3D-printer_Anim" false)
        (`|SpawnActorFromClass` "/Game/OUR_logic/Printing_models/BP_SmallHandler.BP_SmallHandler_C" (`SceneComponent.K2_GetComponentToWorld` (`self.DefaultSceneRoot`)) "Undefined" "OverrideRootScale" null null)
        (`KismetSystemLibrary.Delay` 4.3)
        (`SkeletalMeshComponent.Stop` (`self.3D-printer`))
        (`KismetSystemLibrary.PrintString` "stop")
        (if (== _counter_3 _detail_3)
          _
          (else
            (goto _label_3))))))
  (if (!= _detail_4 0)
    (bind _counter_4 (`/Engine/EditorBlueprintResources/StandardMacros.Do N` _detail_4 :!label _label_4)
      (:`Exit`
        (`SkeletalMeshComponent.PlayAnimation` (`self.3D-printer`) "/Game/OUR_models/3D-printer/3D-printer_Anim.3D-printer_Anim" false)
        (`|SpawnActorFromClass` "/Game/OUR_logic/Printing_models/BP_SmallWheel.BP_SmallWheel_C" (`SceneComponent.K2_GetComponentToWorld` (`self.DefaultSceneRoot`)) "Undefined" "OverrideRootScale" null null)
        (`KismetSystemLibrary.Delay` 4.3)
        (`SkeletalMeshComponent.Stop` (`self.3D-printer`))
        (`KismetSystemLibrary.PrintString` "stop")
        (if (== _counter_4 _detail_4)
          _
          (else
            (goto _label_4))))))
  (if (!= _detail_5 0)
    (bind _counter_5 (`/Engine/EditorBlueprintResources/StandardMacros.Do N` _detail_5 :!label _label_5)
      (:`Exit`
        (`SkeletalMeshComponent.PlayAnimation` (`self.3D-printer`) "/Game/OUR_models/3D-printer/3D-printer_Anim.3D-printer_Anim" false)
        (`|SpawnActorFromClass` "/Game/OUR_logic/Printing_models/BP_SmallWheelAxe.BP_SmallWheelAxe_C" (`SceneComponent.K2_GetComponentToWorld` (`self.DefaultSceneRoot`)) "Undefined" "OverrideRootScale" null null)
        (`KismetSystemLibrary.Delay` 4.3)
        (`SkeletalMeshComponent.Stop` (`self.3D-printer`))
        (`KismetSystemLibrary.PrintString` "stop")
        (if (== _counter_5 _detail_5)
          _
          (else
            (goto _label_5))))))
  (if (!= _detail_6 0)
    (bind _counter_6 (`/Engine/EditorBlueprintResources/StandardMacros.Do N` _detail_6 :!label _label_6)
      (:`Exit`
        (`SkeletalMeshComponent.PlayAnimation` (`self.3D-printer`) "/Game/OUR_models/3D-printer/3D-printer_Anim.3D-printer_Anim" false)
        (`|SpawnActorFromClass` "/Game/OUR_logic/Printing_models/BP_Wheel.BP_Wheel_C" (`SceneComponent.K2_GetComponentToWorld` (`self.DefaultSceneRoot`)) "Undefined" "OverrideRootScale" null null)
        (`KismetSystemLibrary.Delay` 4.3)
        (`SkeletalMeshComponent.Stop` (`self.3D-printer`))
        (`KismetSystemLibrary.PrintString` "stop")
        (if (== _counter_6 _detail_6)
          _
          (else
            (goto _label_6))))))
  (`Widget.SetVisibility` (stale `OK` _returnvalue) "Visible"))

(event `Reset_loop`
  (`|ExecutionSequence`
    (:`then_0`
      (goto _label :!via `Reset`))
    (:`then_1`
      (goto _label_2 :!via `Reset`))
    (:`then_2`
      (goto _label_3 :!via `Reset`))
    (:`then_3`
      (goto _label_4 :!via `Reset`))
    (:`then_4`
      (goto _label_5 :!via `Reset`))
    (:`then_5`
      (goto _label_6 :!via `Reset`))))

(fn `UserConstructionScript`)