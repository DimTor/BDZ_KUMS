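; BP_sborka lets the player pick up and drag movable components with the mouse while GrabMode is on.
; A left click line-traces from the cursor and stores the hit component and its distance.
; Tick keeps it at that distance along the cursor ray, using a PhysicsHandle for simulating bodies and SetWorldLocation otherwise.
; Releasing the button drops it; the stored relative grab offset is never applied.
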(event `self.ReceiveTick`
  (params (DeltaSeconds :type "Float (single-precision)"))
  (bind _grab_component (`self.Grab_Component`))
  (bind (_worldlocation _worlddirection) (`PlayerController.DeprojectMousePositionToWorld` (`GameplayStatics.GetPlayerController` 0)))
  (bind _returnvalue (+ _worldlocation (* _worlddirection (`self.Original_Distance_to_Object`))))
  (if (`self.Grab_Mode`)
    (if (`KismetSystemLibrary.IsValid` _grab_component)
      (if (`SceneComponent.IsSimulatingPhysics` _grab_component "None")
        (`PhysicsHandleComponent.SetTargetLocation` (`self.PhysicsHandle`) _returnvalue)
        (else
          (`SceneComponent.K2_SetWorldLocation` (`self.Grab_Component`) _returnvalue false false))))))

(event `Key|LeftMouseButton`
  (params (Key :type "Key Structure"))
  (bind _grab_mode (`self.Grab_Mode`))
  (bind (_worldlocation _worlddirection) (`PlayerController.DeprojectMousePositionToWorld` (`GameplayStatics.GetPlayerController` 0)))
  (:`Pressed`
    (if _grab_mode
      (bind _outhit (`KismetSystemLibrary.LineTraceSingle` :`Start` _worldlocation :`End` (+ _worldlocation (* _worlddirection 1000.0)) :`TraceChannel` "TraceTypeQuery1" :`DrawDebugType` "ForDuration" :`DrawTime` 0.0))
      (bind (_bblockinghit _binitialoverlap _time _distance _location _impactpoint _normal _impactnormal _physmat _hitactor _hitcomponent) (`GameplayStatics.BreakHitResult` _outhit))
      (if (`|EnumEquality` (`SceneComponent.Mobility` _hitcomponent) (enumliteral `EComponentMobility` "Movable"))
        (bind _output_get (set `self.Grab_Component` _hitcomponent))
        (set `self.Original_Distance_to_Object` _distance)
        (if (`SceneComponent.IsSimulatingPhysics` _output_get "None")
          (`PhysicsHandleComponent.GrabComponentAtLocation` (`self.PhysicsHandle`) (`self.Grab_Component`) "None" _location)
          (else
            (set `self.Relative_Grab_Location` (`KismetMathLibrary.InverseTransformLocation` (`KismetMathLibrary.Conv_VectorToTransform` _location) (`SceneComponent.K2_GetComponentLocation` _hitcomponent)))))
        (else
          (`KismetSystemLibrary.PrintString` "Stationary")))))
  (:`Released`
    (if _grab_mode
      (set `self.Grab_Component` null)
      (`PhysicsHandleComponent.ReleaseComponent` (`self.PhysicsHandle`)))))

(fn `UserConstructionScript`)