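; BP_scene runs the game's flow, switching cameras between start view, printer stage and assembly (sborka) stage, and handles mouse object grabbing.
; BeginPlay shows the start menu and V opens pause; stage events trigger BP_printer and BP_sborka logic.
; In GrabMode, left click traces from the cursor for Movable components, then Tick drags them at hit distance, via PhysicsHandle if simulating physics, otherwise SetWorldLocation.
; UpdateAllToStart is empty.
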(event `self.ReceiveTick`
  (params (DeltaSeconds :type "Float (single-precision)"))
  (bind _grab_component (`self.Grab_component`))
  (bind (_worldlocation _worlddirection) (`PlayerController.DeprojectMousePositionToWorld` (`GameplayStatics.GetPlayerController` 0)))
  (bind _returnvalue (+ _worldlocation (* _worlddirection (`self.OriginalDistanceToObject`))))
  (if (`self.Grab_Mode`)
    (if (`KismetSystemLibrary.IsValid` _grab_component)
      (if (`SceneComponent.IsSimulatingPhysics` _grab_component "None")
        (`PhysicsHandleComponent.SetTargetLocation` (`self.PhysicsHandle`) _returnvalue)
        (else
          (`SceneComponent.K2_SetWorldLocation` (`self.Grab_component`) _returnvalue false false))))))

(event `Key|LeftMouseButton`
  (params (Key :type "Key Structure"))
  (bind _grab_mode (`self.Grab_Mode`))
  (bind (_worldlocation _worlddirection) (`PlayerController.DeprojectMousePositionToWorld` (`GameplayStatics.GetPlayerController` 0)))
  (:`Pressed`
    (if _grab_mode
      (bind _outhit (`KismetSystemLibrary.LineTraceSingle` :`Start` _worldlocation :`End` (+ _worldlocation (* _worlddirection 1000.0)) :`TraceChannel` "TraceTypeQuery1" :`DrawDebugType` "ForDuration"))
      (bind (_bblockinghit _binitialoverlap _time _distance _location _impactpoint _normal _impactnormal _physmat _hitactor _hitcomponent) (`GameplayStatics.BreakHitResult` _outhit))
      (if (`|EnumEquality` (`SceneComponent.Mobility` _hitcomponent) (enumliteral `EComponentMobility` "Movable"))
        (bind _output_get (set `self.Grab_component` _hitcomponent))
        (set `self.OriginalDistanceToObject` _distance)
        (if (`SceneComponent.IsSimulatingPhysics` _output_get "None")
          (`PhysicsHandleComponent.GrabComponentAtLocation` (`self.PhysicsHandle`) (`self.Grab_component`) "None" _location)
          (else
            (set `self.RelativeGrabLocation` (`KismetMathLibrary.InverseTransformLocation` (`KismetMathLibrary.Conv_VectorToTransform` _location) (`SceneComponent.K2_GetComponentLocation` _hitcomponent))))))))
  (:`Released`
    (if _grab_mode
      (set `self.Grab_component` null)
      (`PhysicsHandleComponent.ReleaseComponent` (`self.PhysicsHandle`)))))

(event `main_view`
  (`ActorComponent.Deactivate` (`self.Camera_for_printer`))
  (`ActorComponent.Deactivate` (`self.Camera_for_sborka`))
  (`ActorComponent.Activate` (`self.Start_camera`) false))

(event `self.ReceiveBeginPlay`
  (`ActorComponent.Activate` (`self.Start_camera`) false)
  (bind _returnvalue (`|CreateWidget` "/Game/OUR_logic/BP_startmenu.BP_startmenu_C"))
  (`UserWidget.AddToViewport` _returnvalue 0)
  (`KismetSystemLibrary.PrintString` "Hello"))

(event `start_game`
  (`self.update_all_to_start`)
  (`ActorComponent.Deactivate` (`self.Start_camera`))
  (`ActorComponent.Activate` (`self.Camera_for_printer`) true)
  (bind _outactors (`GameplayStatics.GetAllActorsOfClass` "/Game/OUR_logic/BP_printer.BP_printer_C"))
  (`/Game/OUR_logic/BP_printer.Printer_logic` _outactors))

(event `Key|V`
  (params (Key :type "Key Structure"))
  (:`Pressed`
    (bind _returnvalue (`|CreateWidget` "/Game/OUR_logic/BP_Pause.BP_Pause_C"))
    (`UserWidget.AddToViewport` _returnvalue 0)))

(event `print_is_ok`
  (`ActorComponent.Activate` (`self.Camera_for_sborka`) false)
  (bind _outactors (`GameplayStatics.GetAllActorsOfClass` "/Game/OUR_logic/BP_sborka.BP_sborka_C"))
  (`/Game/OUR_logic/BP_sborka.Sborka_Logic` _outactors))

(fn `update_all_to_start`)

(fn `UserConstructionScript`)