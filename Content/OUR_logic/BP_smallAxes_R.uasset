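; BP_smallAxes_R is an axle in a chassis assembly task that accepts BP_ved_wheels parts.
; Tick flips the axle once when moved and, once it is stationary and the character's CountOfShassi is 2, activates the placement zone.
; Box overlaps briefly show the Places marker for movable parts.
; Places overlaps snap and lock matching wheels, mirroring the second via negative scale and deactivating, while BP_wheels triggers MakeMistake on the character.
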(event `self.ReceiveBeginPlay`
  (set `self.start_loc` (`SceneComponent.K2_GetComponentLocation` (`self.Axes`))))

(event `self.ReceiveTick`
  (params (DeltaSeconds :type "Float (single-precision)"))
  (bind _places (`self.Places`))
  (if (== (enumliteral `EComponentMobility` "Stationary") (`SceneComponent.Mobility` (`self.Axes`)))
    (bind _returnvalue (`GameplayStatics.GetActorOfClass` "/Game/OUR_logic/BP_character.BP_character_C"))
    (if (== (`/Game/OUR_logic/BP_character.count_of_shassi` _returnvalue) 2)
      (set `self.Is_Active` true)
      (`SceneComponent.SetHiddenInGame` _places false false)
      (`SceneComponent.SetMobility` _places "Stationary")
      (`SceneComponent.SetMobility` (`self.Box`) "Stationary"))
    (elif (`self.horizont`)
      (if (not (== (`self.start_loc`) (`SceneComponent.K2_GetComponentLocation` (`self.Axes`))))
        (`SceneComponent.K2_SetWorldRotation` (`self.Axes`) (struct :`Roll` 180.0) false false)
        (set `self.horizont` false)))))

(event `self.Places.OnComponentBeginOverlap`
  (params (OverlappedComponent :type "PrimitiveComponent Object Reference") (OtherActor :type "Actor Object Reference") (OtherComp :type "PrimitiveComponent Object Reference") (OtherBodyIndex :type Integer) (bFromSweep :type Boolean) (SweepResult :type "HitResult Structure (by ref)"))
  (bind _returnvalue (`GameplayStatics.GetObjectClass` OtherActor))
  (if (`self.Is_Active`)
    (if (`SceneComponent.IsVisible` OtherComp)
      (if (== (`SceneComponent.Mobility` OtherComp) (enumliteral `EComponentMobility` "Movable"))
        (bind _returnvalue_2 (`GameplayStatics.GetActorOfClass` "/Game/OUR_logic/BP_ved_wheels.BP_ved_wheels_C"))
        (if (== (`GameplayStatics.GetObjectClass` _returnvalue_2) _returnvalue)
          (`SceneComponent.K2_SetWorldLocation` OtherComp (`SceneComponent.K2_GetComponentLocation` (`self.Places`)) false false)
          (if (not (== (`self.wheel_count`) 0))
            (`SceneComponent.K2_SetWorldRotation` OtherComp (struct :`Roll` 90.0) false false)
            (`SceneComponent.SetWorldScale3D` OtherComp (0.02 0.02 -0.03))
            (set `self.Is_Active` false))
          (`SceneComponent.K2_SetWorldRotation` OtherComp (struct :`Roll` 90.0) false false)
          (set `self.wheel_count` 1)
          (if true
            (`SceneComponent.SetMobility` (`Actor.RootComponent` OtherActor) "Stationary")
            (`SceneComponent.SetVisibility` (`self.Places`) false false))
          (else
            (`KismetSystemLibrary.PrintString` "Hello")
            (bind _returnvalue_3 (`GameplayStatics.GetActorOfClass` "/Game/OUR_logic/BP_wheels.BP_wheels_C"))
            (if (== (`GameplayStatics.GetObjectClass` _returnvalue_3) _returnvalue)
              (bind _returnvalue_4 (`GameplayStatics.GetActorOfClass` "/Game/OUR_logic/BP_character.BP_character_C"))
              (`/Game/OUR_logic/BP_character.Make_mistake` _returnvalue_4))))))))

(event `self.Box.OnComponentBeginOverlap`
  (params (OverlappedComponent :type "PrimitiveComponent Object Reference") (OtherActor :type "Actor Object Reference") (OtherComp :type "PrimitiveComponent Object Reference") (OtherBodyIndex :type Integer) (bFromSweep :type Boolean) (SweepResult :type "HitResult Structure (by ref)"))
  (bind _places (`self.Places`))
  (if (`self.Is_Active`)
    (if (== (`SceneComponent.Mobility` OtherComp) (enumliteral `EComponentMobility` "Movable"))
      (`SceneComponent.SetVisibility` _places true false)
      (`KismetSystemLibrary.Delay` 2.0)
      (`SceneComponent.SetVisibility` _places false false :!label _label))))

(event `self.Box.OnComponentEndOverlap`
  (params (OverlappedComponent :type "PrimitiveComponent Object Reference") (OtherActor :type "Actor Object Reference") (OtherComp :type "PrimitiveComponent Object Reference") (OtherBodyIndex :type Integer))
  (if (`self.Is_Active`)
    (if (== (`SceneComponent.Mobility` OtherComp) (enumliteral `EComponentMobility` "Movable"))
      (goto _label))))

(fn `UserConstructionScript`)