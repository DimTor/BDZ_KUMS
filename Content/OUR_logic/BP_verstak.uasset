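; BP_verstak is a workbench actor with a snap slot that locks a drone base (BP_base_of_dron) in place.
; While active, a movable component entering Box reveals the Cube1 marker, and leaving Box hides it.
; A visible component overlapping Cube1 from an actor of the drone base's class snaps to Cube1's location.
; That actor's root then becomes Stationary, the marker hides, and IsActive clears, with no reset here.
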(event `self.ReceiveBeginPlay`
  (`SceneComponent.SetMobility` (`self.Cube`) "Stationary")
  (`SceneComponent.SetMobility` (`self.Cube1`) "Stationary"))

(event `self.Box.OnComponentBeginOverlap`
  (params (OverlappedComponent :type "PrimitiveComponent Object Reference") (OtherActor :type "Actor Object Reference") (OtherComp :type "PrimitiveComponent Object Reference") (OtherBodyIndex :type Integer) (bFromSweep :type Boolean) (SweepResult :type "HitResult Structure (by ref)"))
  (if (`self.is active`)
    (if (== (`SceneComponent.Mobility` OtherComp) (enumliteral `EComponentMobility` "Movable"))
      (`SceneComponent.SetVisibility` (`self.Cube1`) true false))))

(event `self.Box.OnComponentEndOverlap`
  (params (OverlappedComponent :type "PrimitiveComponent Object Reference") (OtherActor :type "Actor Object Reference") (OtherComp :type "PrimitiveComponent Object Reference") (OtherBodyIndex :type Integer))
  (`KismetSystemLibrary.PrintString` "Hello")
  (if (== (`SceneComponent.Mobility` OtherComp) (enumliteral `EComponentMobility` "Movable"))
    (`SceneComponent.SetVisibility` (`self.Cube1`) false false)))

(event `self.Cube1.OnComponentBeginOverlap`
  (params (OverlappedComponent :type "PrimitiveComponent Object Reference") (OtherActor :type "Actor Object Reference") (OtherComp :type "PrimitiveComponent Object Reference") (OtherBodyIndex :type Integer) (bFromSweep :type Boolean) (SweepResult :type "HitResult Structure (by ref)"))
  (if (`self.is active`)
    (if (`SceneComponent.IsVisible` OtherComp)
      (bind _returnvalue (`GameplayStatics.GetActorOfClass` "/Game/OUR_logic/BP_base_of_dron.BP_base_of_dron_C"))
      (if (== (`GameplayStatics.GetObjectClass` _returnvalue) (`GameplayStatics.GetObjectClass` OtherActor))
        (`KismetSystemLibrary.PrintString` "vdvd")
        (if true
          (`SceneComponent.K2_SetWorldLocation` OtherComp (`SceneComponent.K2_GetComponentLocation` (`self.Cube1`)) false false)
          (if true
            (`SceneComponent.SetMobility` (`Actor.RootComponent` OtherActor) "Stationary")
            (set `self.is active` false)
            (`SceneComponent.SetVisibility` (`self.Cube1`) false false)))))))

(fn `UserConstructionScript`)