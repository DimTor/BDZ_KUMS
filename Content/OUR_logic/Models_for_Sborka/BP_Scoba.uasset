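; BP_Scoba is an assembly-game bracket that, once its mesh turns Stationary, becomes a target for the final BP_SensorHandler part.
; Box overlaps with movable components briefly reveal the Places hint.
; A visible handler hitting Places when the character counts two brackets is rotated, moved to Location and frozen, all brackets deactivate, and EndOfGame runs.
; Other actor classes trigger MakeMistake; the summed bracket-position midpoint is left unused.
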(event `self.ReceiveTick`
  (params (DeltaSeconds :type "Float (single-precision)"))
  (bind _places (`self.Places`))
  (if (== (enumliteral `EComponentMobility` "Stationary") (`SceneComponent.Mobility` (`self.Scoba`)))
    (if (`self.start`)
      (set `self.Is_active` true)
      (`SceneComponent.SetHiddenInGame` _places false false)
      (`SceneComponent.SetMobility` _places "Stationary")
      (`SceneComponent.SetMobility` (`self.Box`) "Stationary")
      (set `self.start` false))))

(event `self.Box.OnComponentBeginOverlap`
  (params (OverlappedComponent :type "PrimitiveComponent Object Reference") (OtherActor :type "Actor Object Reference") (OtherComp :type "PrimitiveComponent Object Reference") (OtherBodyIndex :type Integer) (bFromSweep :type Boolean) (SweepResult :type "HitResult Structure (by ref)"))
  (bind _places (`self.Places`))
  (if (`self.Is_active`)
    (if (== (`SceneComponent.Mobility` OtherComp) (enumliteral `EComponentMobility` "Movable"))
      (`SceneComponent.SetVisibility` _places true false)
      (`KismetSystemLibrary.Delay` 2.0)
      (`SceneComponent.SetVisibility` _places false false :!label _label))))

(event `self.Places.OnComponentBeginOverlap`
  (params (OverlappedComponent :type "PrimitiveComponent Object Reference") (OtherActor :type "Actor Object Reference") (OtherComp :type "PrimitiveComponent Object Reference") (OtherBodyIndex :type Integer) (bFromSweep :type Boolean) (SweepResult :type "HitResult Structure (by ref)"))
  (if (`self.Is_active`)
    (if (`SceneComponent.IsVisible` OtherComp)
      (if (== (`SceneComponent.Mobility` OtherComp) (enumliteral `EComponentMobility` "Movable"))
        (bind _returnvalue (`GameplayStatics.GetActorOfClass` "/Game/OUR_logic/Models_for_Sborka/BP_SensorHandler.BP_SensorHandler_C"))
        (if (== (`GameplayStatics.GetObjectClass` _returnvalue) (`GameplayStatics.GetObjectClass` OtherActor))
          (bind _returnvalue_2 (`GameplayStatics.GetActorOfClass` "/Game/OUR_logic/BP_character.BP_character_C"))
          (if (== (`/Game/OUR_logic/BP_character.count_scob_in_sborka` _returnvalue_2) 2)
            (bind _outactors (`GameplayStatics.GetAllActorsOfClass` "BP_Scoba_C"))
            (for _array_element _outactors
              (bind _rootcomponent (`Actor.RootComponent` _array_element))
              (if (== (enumliteral `EComponentMobility` "Stationary") (`SceneComponent.Mobility` _rootcomponent))
                (set `self.world_loc` (+ (`SceneComponent.K2_GetComponentLocation` _rootcomponent) (`self.world_loc`)))))
            (`SceneComponent.K2_SetWorldRotation` OtherComp (struct :`Pitch` 180.0 :`Yaw` -90.0 :`Roll` 180.0) false false)
            (`SceneComponent.K2_SetWorldLocation` OtherComp (`self.location`) false false)
            (if true
              (`SceneComponent.SetMobility` (`Actor.RootComponent` OtherActor) "Stationary")
              (bind _outactors_2 (`GameplayStatics.GetAllActorsOfClass` "BP_Scoba_C"))
              (for _array_element_2 _outactors_2
                (set `/Game/OUR_logic/Models_for_Sborka/BP_Scoba.Is_active` false _array_element_2)
                (`SceneComponent.SetVisibility` (`/Game/OUR_logic/Models_for_Sborka/BP_Scoba.Places` _array_element_2) false false))
              (bind _returnvalue_3 (`GameplayStatics.GetActorOfClass` "/Game/OUR_logic/BP_character.BP_character_C"))
              (`/Game/OUR_logic/BP_character.End_of_game` _returnvalue_3)))
          (else
            (bind _returnvalue_4 (`GameplayStatics.GetActorOfClass` "/Game/OUR_logic/BP_character.BP_character_C"))
            (`/Game/OUR_logic/BP_character.Make_mistake` _returnvalue_4)))))))

(event `self.Box.OnComponentEndOverlap`
  (params (OverlappedComponent :type "PrimitiveComponent Object Reference") (OtherActor :type "Actor Object Reference") (OtherComp :type "PrimitiveComponent Object Reference") (OtherBodyIndex :type Integer))
  (if (`self.Is_active`)
    (if (== (`SceneComponent.Mobility` OtherComp) (enumliteral `EComponentMobility` "Movable"))
      (goto _label))))

(fn `UserConstructionScript`)