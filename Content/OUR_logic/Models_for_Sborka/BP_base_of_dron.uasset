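; Drone base for an assembly game, where parts such as motors, encoders, boards and brackets snap into placeholder slots.
; Tick activates the slots once Cube2 turns Stationary, and enables the ESP32 slot after PowerUp and driver are placed if STOP is set.
; A movable part entering Box briefly reveals open slots.
; Slot overlaps check the part's class, snap and lock it via Stationary mobility, then report to BP_character through EndOfGame and counters.
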(event `self.ReceiveTick`
  (params (DeltaSeconds :type "Float (single-precision)"))
  (bind _places (`self.Places`))
  (if (== (enumliteral `EComponentMobility` "Stationary") (`SceneComponent.Mobility` (`self.Cube2`)))
    (if (`self.start`)
      (set `self.is_active` true)
      (`SceneComponent.SetHiddenInGame` _places false false)
      (`SceneComponent.SetHiddenInGame` (`self.Places2`) false false)
      (`SceneComponent.SetHiddenInGame` (`self.Places3`) false false)
      (`SceneComponent.SetHiddenInGame` (`self.Places_encod1`) false false)
      (`SceneComponent.SetHiddenInGame` (`self.Places_encod2`) false false)
      (`SceneComponent.SetHiddenInGame` (`self.Places_esp`) false false)
      (`SceneComponent.SetHiddenInGame` (`self.podstavka_shassi`) false false)
      (`SceneComponent.SetHiddenInGame` (`self.scoba_place2`) false false)
      (`SceneComponent.SetHiddenInGame` (`self.scoba_place`) false false)
      (`SceneComponent.SetHiddenInGame` (`self.Places_draiver`) false false)
      (`SceneComponent.SetHiddenInGame` (`self.Places_power_up`) false false)
      (`SceneComponent.SetHiddenInGame` (`self.Places_power_down`) false false)
      (`SceneComponent.SetHiddenInGame` (`self.Places_rangefinder`) false false)
      (`SceneComponent.SetMobility` _places "Stationary")
      (`SceneComponent.SetMobility` (`self.Box`) "Stationary")
      (`SceneComponent.SetMobility` (`self.Places3`) "Stationary")
      (`SceneComponent.SetMobility` (`self.Places2`) "Stationary")
      (`SceneComponent.SetMobility` (`self.Places_encod2`) "Stationary")
      (`SceneComponent.SetMobility` (`self.Places_encod1`) "Stationary")
      (`SceneComponent.SetMobility` (`self.Places_esp`) "Stationary")
      (`SceneComponent.SetMobility` (`self.podstavka_shassi`) "Stationary")
      (`SceneComponent.SetMobility` (`self.scoba_place2`) "Stationary")
      (`SceneComponent.SetMobility` (`self.scoba_place`) "Stationary")
      (`SceneComponent.SetMobility` (`self.Places_draiver`) "Stationary")
      (`SceneComponent.SetMobility` (`self.Places_power_up`) "Stationary")
      (`SceneComponent.SetMobility` (`self.Places_power_down`) "Stationary")
      (`SceneComponent.SetMobility` (`self.Places_rangefinder`) "Stationary")
      (set `self.start` false)
      (elif (`self.STOP`)
        (if (not (or (`self.is_active_power_up`) (`self.is_active_driver`) (`self.is_active_power_up`)))
          (set `self.is_active_esp` true)
          (set `self.STOP` false))))))

(event `self.Places.OnComponentBeginOverlap`
  (params (OverlappedComponent :type "PrimitiveComponent Object Reference") (OtherActor :type "Actor Object Reference") (OtherComp :type "PrimitiveComponent Object Reference") (OtherBodyIndex :type Integer) (bFromSweep :type Boolean) (SweepResult :type "HitResult Structure (by ref)"))
  (bind _rootcomponent (`Actor.RootComponent` OtherActor))
  (if (`self.is_active`)
    (if (`self.is_active_wheels1`)
      (if (`SceneComponent.IsVisible` OtherComp)
        (bind _returnvalue (`GameplayStatics.GetActorOfClass` "/Game/OUR_logic/Models_for_Sborka/BP_motor.BP_motor_C"))
        (if (== (`GameplayStatics.GetObjectClass` _returnvalue) (`GameplayStatics.GetObjectClass` OtherActor))
          (`SceneComponent.K2_SetWorldLocation` OtherComp (`SceneComponent.K2_GetComponentLocation` (`self.Places`)) false false)
          (`SceneComponent.K2_SetRelativeRotation` _rootcomponent (struct :`Yaw` 90.0) false false)
          (if true
            (`SceneComponent.SetMobility` _rootcomponent "Stationary")
            (bind _returnvalue_2 (`GameplayStatics.GetActorOfClass` "/Game/OUR_logic/BP_character.BP_character_C"))
            (`/Game/OUR_logic/BP_character.End_of_game` _returnvalue_2)
            (set `self.is_active_wheels1` false)
            (`SceneComponent.SetVisibility` (`self.Places`) false false :!label _label)
            (`SceneComponent.SetVisibility` (`self.Places2`) false false)
            (`SceneComponent.SetVisibility` (`self.Places3`) false false)
            (`SceneComponent.SetVisibility` (`self.Places_encod1`) false false)
            (`SceneComponent.SetVisibility` (`self.Places_encod2`) false false)
            (`SceneComponent.SetVisibility` (`self.Places_power_down`) false false)
            (`SceneComponent.SetVisibility` (`self.Places_power_up`) false false)
            (`SceneComponent.SetVisibility` (`self.Places_draiver`) false false)
            (`SceneComponent.SetVisibility` (`self.scoba_place`) false false)
            (`SceneComponent.SetVisibility` (`self.scoba_place2`) false false)
            (`SceneComponent.SetVisibility` (`self.podstavka_shassi`) false false)
            (`SceneComponent.SetVisibility` (`self.Places_esp`) false false)
            (`SceneComponent.SetVisibility` (`self.Places_rangefinder`) false false))
          (else
            (`KismetSystemLibrary.PrintString` "")))))))

(event `self.Box.OnComponentBeginOverlap`
  (params (OverlappedComponent :type "PrimitiveComponent Object Reference") (OtherActor :type "Actor Object Reference") (OtherComp :type "PrimitiveComponent Object Reference") (OtherBodyIndex :type Integer) (bFromSweep :type Boolean) (SweepResult :type "HitResult Structure (by ref)"))
  (bind _returnvalue (== (`SceneComponent.Mobility` OtherComp) (enumliteral `EComponentMobility` "Movable")))
  (if (`self.is_active`)
    (if _returnvalue
      (if (`self.is_active_wheels1`)
        (`SceneComponent.SetVisibility` (`self.Places`) true false))
      (if (`self.is_active_wheels2`)
        (`SceneComponent.SetVisibility` (`self.Places2`) true false))
      (if (`self.is_active_wheels3`)
        (`SceneComponent.SetVisibility` (`self.Places3`) true false))
      (if (`self.is_active_enc1`)
        (`SceneComponent.SetVisibility` (`self.Places_encod1`) true false))
      (if (`self.is_actov_enc2`)
        (`SceneComponent.SetVisibility` (`self.Places_encod2`) true false))
      (if (`self.is_active_power_down`)
        (`SceneComponent.SetVisibility` (`self.Places_power_down`) true false))
      (if (`self.is_active_power_up`)
        (`SceneComponent.SetVisibility` (`self.Places_power_up`) true false))
      (if (`self.is_active_driver`)
        (`SceneComponent.SetVisibility` (`self.Places_draiver`) true false))
      (if (`self.is_active_scoba`)
        (`SceneComponent.SetVisibility` (`self.scoba_place`) true false))
      (if (`self.is_active_scoba2`)
        (`SceneComponent.SetVisibility` (`self.scoba_place2`) true false))
      (if (`self.is_active_shassi_place`)
        (`SceneComponent.SetVisibility` (`self.podstavka_shassi`) true false))
      (if (`self.is_active_esp`)
        (`SceneComponent.SetVisibility` (`self.Places_esp`) true false))
      (if (`self.IS_Actife_dalnomer`)
        (`SceneComponent.SetVisibility` (`self.Places_rangefinder`) true false))
      (if _returnvalue
        (`KismetSystemLibrary.Delay` 5.0)
        (goto _label)
        (else
          (goto _label))))))

(event `self.Places2.OnComponentBeginOverlap`
  (params (OverlappedComponent :type "PrimitiveComponent Object Reference") (OtherActor :type "Actor Object Reference") (OtherComp :type "PrimitiveComponent Object Reference") (OtherBodyIndex :type Integer) (bFromSweep :type Boolean) (SweepResult :type "HitResult Structure (by ref)"))
  (if (`self.is_active`)
    (if (`self.is_active_wheels2`)
      (if (`SceneComponent.IsVisible` OtherComp)
        (bind _returnvalue (`GameplayStatics.GetActorOfClass` "/Game/OUR_logic/Models_for_Sborka/BP_motor.BP_motor_C"))
        (if (== (`GameplayStatics.GetObjectClass` _returnvalue) (`GameplayStatics.GetObjectClass` OtherActor))
          (`SceneComponent.K2_SetWorldLocation` OtherComp (`SceneComponent.K2_GetComponentLocation` (`self.Places2`)) false false)
          (`SceneComponent.K2_SetRelativeRotation` (`Actor.RootComponent` OtherActor) (struct :`Yaw` -90.0) false false)
          (if true
            (`SceneComponent.SetMobility` (`Actor.RootComponent` OtherActor) "Stationary")
            (bind _returnvalue_2 (`GameplayStatics.GetActorOfClass` "/Game/OUR_logic/BP_character.BP_character_C"))
            (`/Game/OUR_logic/BP_character.End_of_game` _returnvalue_2)
            (set `self.is_active_wheels2` false)
            (goto _label))
          (else
            (`KismetSystemLibrary.PrintString` "")))))))

(event `self.Places3.OnComponentBeginOverlap`
  (params (OverlappedComponent :type "PrimitiveComponent Object Reference") (OtherActor :type "Actor Object Reference") (OtherComp :type "PrimitiveComponent Object Reference") (OtherBodyIndex :type Integer) (bFromSweep :type Boolean) (SweepResult :type "HitResult Structure (by ref)"))
  (if (`self.is_active`)
    (if (`self.is_active_wheels3`)
      (if (`SceneComponent.IsVisible` OtherComp)
        (bind _returnvalue (`GameplayStatics.GetActorOfClass` "/Game/OUR_logic/Models_for_Sborka/BP_BatteryHolder.BP_BatteryHolder_C"))
        (if (== (`GameplayStatics.GetObjectClass` _returnvalue) (`GameplayStatics.GetObjectClass` OtherActor))
          (`SceneComponent.K2_SetWorldLocation` OtherComp (+ (`SceneComponent.K2_GetComponentLocation` (`self.Places3`)) (0.0 9.0 -5.0)) false false)
          (`SceneComponent.K2_SetWorldRotation` :`self` OtherComp)
          (if true
            (`SceneComponent.SetMobility` (`Actor.RootComponent` OtherActor) "Stationary")
            (bind _returnvalue_2 (`GameplayStatics.GetActorOfClass` "/Game/OUR_logic/BP_character.BP_character_C"))
            (`/Game/OUR_logic/BP_character.End_of_game` _returnvalue_2)
            (set `self.is_active_wheels3` false)
            (goto _label))
          (else
            (`KismetSystemLibrary.PrintString` "")))))))

(event `self.Box.OnComponentEndOverlap`
  (params (OverlappedComponent :type "PrimitiveComponent Object Reference") (OtherActor :type "Actor Object Reference") (OtherComp :type "PrimitiveComponent Object Reference") (OtherBodyIndex :type Integer))
  (if (`self.is_active`)
    (if (== (`SceneComponent.Mobility` OtherComp) (enumliteral `EComponentMobility` "Movable"))
      (goto _label))))

(event `self.Places_encod1.OnComponentBeginOverlap`
  (params (OverlappedComponent :type "PrimitiveComponent Object Reference") (OtherActor :type "Actor Object Reference") (OtherComp :type "PrimitiveComponent Object Reference") (OtherBodyIndex :type Integer) (bFromSweep :type Boolean) (SweepResult :type "HitResult Structure (by ref)"))
  (bind _rootcomponent (`Actor.RootComponent` OtherActor))
  (if (`self.is_active`)
    (if (`self.is_active_enc1`)
      (if (`SceneComponent.IsVisible` OtherComp)
        (bind _returnvalue (`GameplayStatics.GetActorOfClass` "/Game/OUR_logic/Models_for_Sborka/BP_encoder.BP_encoder_C"))
        (if (== (`GameplayStatics.GetObjectClass` _returnvalue) (`GameplayStatics.GetObjectClass` OtherActor))
          (`SceneComponent.K2_SetWorldLocation` OtherComp (`SceneComponent.K2_GetComponentLocation` (`self.Places_encod1`)) false false)
          (`SceneComponent.K2_SetRelativeRotation` _rootcomponent (struct :`Yaw` 180.0 :`Roll` 180.0) false false)
          (if true
            (`SceneComponent.SetMobility` _rootcomponent "Stationary")
            (set `self.is_active_enc1` false)
            (bind _returnvalue_2 (`GameplayStatics.GetActorOfClass` "/Game/OUR_logic/BP_character.BP_character_C"))
            (`/Game/OUR_logic/BP_character.End_of_game` _returnvalue_2)
            (goto _label))
          (else
            (`KismetSystemLibrary.PrintString` "")))))))

(event `self.Places_encod2.OnComponentBeginOverlap`
  (params (OverlappedComponent :type "PrimitiveComponent Object Reference") (OtherActor :type "Actor Object Reference") (OtherComp :type "PrimitiveComponent Object Reference") (OtherBodyIndex :type Integer) (bFromSweep :type Boolean) (SweepResult :type "HitResult Structure (by ref)"))
  (bind _rootcomponent (`Actor.RootComponent` OtherActor))
  (if (`self.is_active`)
    (if (`self.is_actov_enc2`)
      (if (`SceneComponent.IsVisible` OtherComp)
        (bind _returnvalue (`GameplayStatics.GetActorOfClass` "/Game/OUR_logic/Models_for_Sborka/BP_encoder.BP_encoder_C"))
        (if (== (`GameplayStatics.GetObjectClass` _returnvalue) (`GameplayStatics.GetObjectClass` OtherActor))
          (`SceneComponent.K2_SetWorldLocation` OtherComp (`SceneComponent.K2_GetComponentLocation` (`self.Places_encod2`)) false false)
          (`SceneComponent.K2_SetRelativeRotation` _rootcomponent (struct :`Yaw` 180.0 :`Roll` 180.0) false false)
          (if true
            (`SceneComponent.SetMobility` _rootcomponent "Stationary")
            (bind _returnvalue_2 (`GameplayStatics.GetActorOfClass` "/Game/OUR_logic/BP_character.BP_character_C"))
            (`/Game/OUR_logic/BP_character.End_of_game` _returnvalue_2)
            (set `self.is_actov_enc2` false)
            (goto _label))
          (else
            (`KismetSystemLibrary.PrintString` "")))))))

(event `self.scoba_place.OnComponentBeginOverlap`
  (params (OverlappedComponent :type "PrimitiveComponent Object Reference") (OtherActor :type "Actor Object Reference") (OtherComp :type "PrimitiveComponent Object Reference") (OtherBodyIndex :type Integer) (bFromSweep :type Boolean) (SweepResult :type "HitResult Structure (by ref)"))
  (if (`self.is_active`)
    (if (`self.is_active_scoba`)
      (if (`SceneComponent.IsVisible` OtherComp)
        (bind _returnvalue (`GameplayStatics.GetActorOfClass` "/Game/OUR_logic/Models_for_Sborka/BP_Scoba.BP_Scoba_C"))
        (if (== (`GameplayStatics.GetObjectClass` _returnvalue) (`GameplayStatics.GetObjectClass` OtherActor))
          (`SceneComponent.K2_SetWorldLocation` OtherComp (`SceneComponent.K2_GetComponentLocation` (`self.scoba_place`)) false false)
          (if true
            (`SceneComponent.SetMobility` (`Actor.RootComponent` OtherActor) "Stationary")
            (set `self.is_active_scoba` false)
            (bind _returnvalue_2 (`GameplayStatics.GetActorOfClass` "/Game/OUR_logic/BP_character.BP_character_C" :!label _label_2))
            (`/Game/OUR_logic/BP_character.End_of_game` _returnvalue_2)
            (`/Game/OUR_logic/BP_character.cout_scob` _returnvalue_2)
            (goto _label))
          (else
            (`KismetSystemLibrary.PrintString` "")))))))

(event `self.scoba_place2.OnComponentBeginOverlap`
  (params (OverlappedComponent :type "PrimitiveComponent Object Reference") (OtherActor :type "Actor Object Reference") (OtherComp :type "PrimitiveComponent Object Reference") (OtherBodyIndex :type Integer) (bFromSweep :type Boolean) (SweepResult :type "HitResult Structure (by ref)"))
  (if (`self.is_active`)
    (if (`self.is_active_scoba2`)
      (if (`SceneComponent.IsVisible` OtherComp)
        (bind _returnvalue (`GameplayStatics.GetActorOfClass` "/Game/OUR_logic/Models_for_Sborka/BP_Scoba.BP_Scoba_C"))
        (if (== (`GameplayStatics.GetObjectClass` _returnvalue) (`GameplayStatics.GetObjectClass` OtherActor))
          (`SceneComponent.K2_SetWorldLocation` OtherComp (`SceneComponent.K2_GetComponentLocation` (`self.scoba_place2`)) false false)
          (if true
            (`SceneComponent.SetMobility` (`Actor.RootComponent` OtherActor) "Stationary")
            (set `self.is_active_scoba2` false)
            (goto _label_2))
          (else
            (`KismetSystemLibrary.PrintString` "")))))))

(event `self.podstavka_shassi.OnComponentBeginOverlap`
  (params (OverlappedComponent :type "PrimitiveComponent Object Reference") (OtherActor :type "Actor Object Reference") (OtherComp :type "PrimitiveComponent Object Reference") (OtherBodyIndex :type Integer) (bFromSweep :type Boolean) (SweepResult :type "HitResult Structure (by ref)"))
  (if (`self.is_active`)
    (if (`self.is_active_shassi_place`)
      (if (`SceneComponent.IsVisible` OtherComp)
        (bind _returnvalue (`GameplayStatics.GetActorOfClass` "/Game/OUR_logic/Models_for_Sborka/BP_smallAxes_L.BP_smallAxes_L_C"))
        (bind _returnvalue_2 (`GameplayStatics.GetActorOfClass` "/Game/OUR_logic/Models_for_Sborka/BP_smallAxes_R.BP_smallAxes_R_C"))
        (if (and (`self.is_left`) (== (`GameplayStatics.GetObjectClass` _returnvalue) (`GameplayStatics.GetObjectClass` OtherActor)))
          (set `self.is_left` false)
          (`SceneComponent.K2_SetWorldLocation` OtherComp (`SceneComponent.K2_GetComponentLocation` (`self.podstavka_shassi`)) false false :!label _label_3)
          (if true
            (`SceneComponent.SetMobility` (`Actor.RootComponent` OtherActor) "Stationary")
            (bind _returnvalue_3 (`GameplayStatics.GetActorOfClass` "/Game/OUR_logic/BP_character.BP_character_C"))
            (`/Game/OUR_logic/BP_character.End_of_game` _returnvalue_3)
            (bind _returnvalue_4 (== 2 (`/Game/OUR_logic/BP_character.count_of_shassi` _returnvalue_3)))
            (if (not _returnvalue_4)
              (`/Game/OUR_logic/BP_character.Count_shassi` _returnvalue_3)
              (if _returnvalue_4
                _
                (else
                  (goto _label))))
            (set `self.is_active_shassi_place` false)
            (goto _label))
          (elif (and (== (`GameplayStatics.GetObjectClass` _returnvalue_2) (`GameplayStatics.GetObjectClass` OtherActor)) (`self.is_right`))
            (set `self.is_right` false)
            (goto _label_3)
            (else
              (`KismetSystemLibrary.PrintString` ""))))))))

(event `self.Places_power_up.OnComponentBeginOverlap`
  (params (OverlappedComponent :type "PrimitiveComponent Object Reference") (OtherActor :type "Actor Object Reference") (OtherComp :type "PrimitiveComponent Object Reference") (OtherBodyIndex :type Integer) (bFromSweep :type Boolean) (SweepResult :type "HitResult Structure (by ref)"))
  (bind _rootcomponent (`Actor.RootComponent` OtherActor))
  (if (`self.is_active`)
    (if (`self.is_active_power_up`)
      (if (`SceneComponent.IsVisible` OtherComp)
        (bind _returnvalue (`GameplayStatics.GetActorOfClass` "/Game/OUR_logic/Models_for_Sborka/BP_PowerUP.BP_PowerUP_C"))
        (if (== (`GameplayStatics.GetObjectClass` _returnvalue) (`GameplayStatics.GetObjectClass` OtherActor))
          (`SceneComponent.K2_SetWorldLocation` OtherComp (+ (`SceneComponent.K2_GetComponentLocation` (`self.Places_power_up`)) (40.0 0.0 -10.0)) false false)
          (`SceneComponent.K2_SetRelativeRotation` _rootcomponent (struct :`Yaw` 180.0) false false)
          (if true
            (`SceneComponent.SetMobility` _rootcomponent "Stationary")
            (set `self.is_active_power_up` false)
            (bind _returnvalue_2 (`GameplayStatics.GetActorOfClass` "/Game/OUR_logic/BP_character.BP_character_C"))
            (`/Game/OUR_logic/BP_character.End_of_game` _returnvalue_2)
            (goto _label))
          (else
            (`KismetSystemLibrary.PrintString` "")))))))

(event `self.Places_power_down.OnComponentBeginOverlap`
  (params (OverlappedComponent :type "PrimitiveComponent Object Reference") (OtherActor :type "Actor Object Reference") (OtherComp :type "PrimitiveComponent Object Reference") (OtherBodyIndex :type Integer) (bFromSweep :type Boolean) (SweepResult :type "HitResult Structure (by ref)"))
  (bind _rootcomponent (`Actor.RootComponent` OtherActor))
  (if (`self.is_active`)
    (if (`self.is_active_power_down`)
      (if (`SceneComponent.IsVisible` OtherComp)
        (bind _returnvalue (`GameplayStatics.GetActorOfClass` "/Game/OUR_logic/Models_for_Sborka/BP_PowerDown.BP_PowerDown_C"))
        (if (== (`GameplayStatics.GetObjectClass` _returnvalue) (`GameplayStatics.GetObjectClass` OtherActor))
          (`SceneComponent.K2_SetWorldLocation` OtherComp (+ (`SceneComponent.K2_GetComponentLocation` (`self.Places_power_down`)) (0.0 0.0 14.0)) false false)
          (`SceneComponent.K2_SetRelativeRotation` _rootcomponent (struct :`Yaw` 180.0) false false)
          (if true
            (`SceneComponent.SetMobility` _rootcomponent "Stationary")
            (set `self.is_active_power_down` false)
            (bind _returnvalue_2 (`GameplayStatics.GetActorOfClass` "/Game/OUR_logic/BP_character.BP_character_C"))
            (`/Game/OUR_logic/BP_character.End_of_game` _returnvalue_2)
            (goto _label))
          (else
            (`KismetSystemLibrary.PrintString` "")))))))

(event `self.Places_draiver.OnComponentBeginOverlap`
  (params (OverlappedComponent :type "PrimitiveComponent Object Reference") (OtherActor :type "Actor Object Reference") (OtherComp :type "PrimitiveComponent Object Reference") (OtherBodyIndex :type Integer) (bFromSweep :type Boolean) (SweepResult :type "HitResult Structure (by ref)"))
  (bind _rootcomponent (`Actor.RootComponent` OtherActor))
  (if (`self.is_active`)
    (if (`self.is_active_driver`)
      (if (`SceneComponent.IsVisible` OtherComp)
        (bind _returnvalue (`GameplayStatics.GetActorOfClass` "/Game/OUR_logic/Models_for_Sborka/BP_Draiver.BP_Draiver_C"))
        (if (== (`GameplayStatics.GetObjectClass` _returnvalue) (`GameplayStatics.GetObjectClass` OtherActor))
          (`SceneComponent.K2_SetWorldLocation` OtherComp (+ (`SceneComponent.K2_GetComponentLocation` (`self.Places_draiver`)) (2.0 4.0 -3.0)) false false)
          (`SceneComponent.K2_SetRelativeRotation` _rootcomponent (struct :`Pitch` 180.0 :`Yaw` 180.0) false false)
          (if true
            (`SceneComponent.SetMobility` _rootcomponent "Stationary")
            (set `self.is_active_driver` false)
            (bind _returnvalue_2 (`GameplayStatics.GetActorOfClass` "/Game/OUR_logic/BP_character.BP_character_C"))
            (`/Game/OUR_logic/BP_character.End_of_game` _returnvalue_2)
            (goto _label))
          (else
            (`KismetSystemLibrary.PrintString` "")))))))

(event `self.Places_rangefinder.OnComponentBeginOverlap`
  (params (OverlappedComponent :type "PrimitiveComponent Object Reference") (OtherActor :type "Actor Object Reference") (OtherComp :type "PrimitiveComponent Object Reference") (OtherBodyIndex :type Integer) (bFromSweep :type Boolean) (SweepResult :type "HitResult Structure (by ref)"))
  (bind _rootcomponent (`Actor.RootComponent` OtherActor))
  (if (`self.is_active`)
    (if (`self.IS_Actife_dalnomer`)
      (if (`SceneComponent.IsVisible` OtherComp)
        (bind _returnvalue (`GameplayStatics.GetActorOfClass` "/Game/OUR_logic/Models_for_Sborka/BP_rangefinder.BP_rangefinder_C"))
        (if (== (`GameplayStatics.GetObjectClass` _returnvalue) (`GameplayStatics.GetObjectClass` OtherActor))
          (`SceneComponent.K2_SetWorldLocation` OtherComp (+ (`SceneComponent.K2_GetComponentLocation` (`self.Places_rangefinder`)) (2.0 -10.0 -3.0)) false false)
          (`SceneComponent.K2_SetRelativeRotation` _rootcomponent (struct :`Yaw` 90.0 :`Roll` -180.0) false false)
          (if true
            (`SceneComponent.SetMobility` _rootcomponent "Stationary")
            (set `self.IS_Actife_dalnomer` false)
            (bind _returnvalue_2 (`GameplayStatics.GetActorOfClass` "/Game/OUR_logic/BP_character.BP_character_C"))
            (`/Game/OUR_logic/BP_character.End_of_game` _returnvalue_2)
            (goto _label))
          (else
            (`KismetSystemLibrary.PrintString` "")))))))

(event `self.Places_esp.OnComponentBeginOverlap`
  (params (OverlappedComponent :type "PrimitiveComponent Object Reference") (OtherActor :type "Actor Object Reference") (OtherComp :type "PrimitiveComponent Object Reference") (OtherBodyIndex :type Integer) (bFromSweep :type Boolean) (SweepResult :type "HitResult Structure (by ref)"))
  (bind _rootcomponent (`Actor.RootComponent` OtherActor))
  (if (`self.is_active`)
    (if (`self.is_active_esp`)
      (if (`SceneComponent.IsVisible` OtherComp)
        (bind _returnvalue (`GameplayStatics.GetActorOfClass` "/Game/OUR_logic/Models_for_Sborka/BP_esp32.BP_esp32_C"))
        (if (== (`GameplayStatics.GetObjectClass` _returnvalue) (`GameplayStatics.GetObjectClass` OtherActor))
          (`SceneComponent.K2_SetWorldLocation` OtherComp (+ (`SceneComponent.K2_GetComponentLocation` (`self.Places_esp`)) (35.0 20.0 -20.0)) false false)
          (`SceneComponent.K2_SetRelativeRotation` _rootcomponent (struct :`Yaw` -90.0 :`Roll` 90.0) false false)
          (if true
            (`SceneComponent.SetMobility` _rootcomponent "Stationary")
            (set `self.is_active_esp` false)
            (bind _returnvalue_2 (`GameplayStatics.GetActorOfClass` "/Game/OUR_logic/BP_character.BP_character_C"))
            (`/Game/OUR_logic/BP_character.End_of_game` _returnvalue_2)
            (goto _label))
          (else
            (`KismetSystemLibrary.PrintString` "")))))))

(fn `UserConstructionScript`)