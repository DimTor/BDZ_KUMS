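; BP_smallAxes_L is an axes model Blueprint that reorients its Axes component once it is moved from its starting position.
; BeginPlay caches the component's world location.
; While Horizont is set and the component is not Stationary, Tick compares the current location to that start.
; On the first difference it snaps the world rotation to a fixed half-turn and clears Horizont, so the change happens only once.
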(event `self.ReceiveBeginPlay`
  (set `self.start_loc` (`SceneComponent.K2_GetComponentLocation` (`self.Axes`))))

(event `self.ReceiveTick`
  (params (DeltaSeconds :type "Float (single-precision)"))
  (if (== (enumliteral `EComponentMobility` "Stationary") (`SceneComponent.Mobility` (`self.Axes`)))
    _
    (elif (`self.horizont`)
      (if (not (== (`self.start_loc`) (`SceneComponent.K2_GetComponentLocation` (`self.Axes`))))
        (`SceneComponent.K2_SetWorldRotation` (`self.Axes`) (struct :`Roll` 180.0) false false)
        (set `self.horizont` false)))))

(fn `UserConstructionScript`)